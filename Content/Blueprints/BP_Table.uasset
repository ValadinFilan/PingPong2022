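; BP_Table is a table-tennis-style table that spawns balls, tracks which player receives and keeps both players' scores.
; SpawnNewBall drops the configured ball type at a randomized offset, links it to the table and makes player one the receiver.
; Player boxes and table bounds forward overlap events to BP_Ball or BP_AIBall.
; Receiver or thrower loss functions award the point and push scores to the GameMode.
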(event `self.ReceiveBeginPlay`
  (`self.SpawnNewBall`))

(event `self.ReceiveTick`
  (params (DeltaSeconds :type "Float (single-precision)")))

(event `self.PlayerTwoBox.OnComponentBeginOverlap`
  (params (OverlappedComponent :type "PrimitiveComponent Object Reference") (OtherActor :type "Actor Object Reference") (OtherComp :type "PrimitiveComponent Object Reference") (OtherBodyIndex :type Integer) (bFromSweep :type Boolean) (SweepResult :type "HitResult Structure (by ref)"))
  (bind _asbp_ball (cast `/Game/Blueprints/BP_Ball` OtherActor)
    (:`then`
      (`/Game/Blueprints/BP_Ball.EnterTriggerTwo` _asbp_ball))
    (:`CastFailed`
      (bind _asbp_aiball (cast `/Game/Blueprints/BP_AIBall` OtherActor))
      (`/Game/Blueprints/BP_AIBall.EnterTriggerTwo` _asbp_aiball))))

(event `self.PlayerOneBox.OnComponentBeginOverlap`
  (params (OverlappedComponent :type "PrimitiveComponent Object Reference") (OtherActor :type "Actor Object Reference") (OtherComp :type "PrimitiveComponent Object Reference") (OtherBodyIndex :type Integer) (bFromSweep :type Boolean) (SweepResult :type "HitResult Structure (by ref)"))
  (bind _asbp_ball (cast `/Game/Blueprints/BP_Ball` OtherActor)
    (:`then`
      (`/Game/Blueprints/BP_Ball.EnterTriggerOne` _asbp_ball))
    (:`CastFailed`
      (bind _asbp_aiball (cast `/Game/Blueprints/BP_AIBall` OtherActor))
      (`/Game/Blueprints/BP_AIBall.EnterTriggerOne` _asbp_aiball))))

(event `self.TableBox.OnComponentEndOverlap`
  (params (OverlappedComponent :type "PrimitiveComponent Object Reference") (OtherActor :type "Actor Object Reference") (OtherComp :type "PrimitiveComponent Object Reference") (OtherBodyIndex :type Integer))
  (bind _asbp_ball (cast `/Game/Blueprints/BP_Ball` OtherActor)
    (:`then`
      (`/Game/Blueprints/BP_Ball.OutOfTable` _asbp_ball))
    (:`CastFailed`
      (bind _asbp_aiball (cast `/Game/Blueprints/BP_AIBall` OtherActor))
      (`/Game/Blueprints/BP_AIBall.OutOfTable` _asbp_aiball))))

(event `self.NetMesh.OnComponentHit`
  (params (HitComponent :type "PrimitiveComponent Object Reference") (OtherActor :type "Actor Object Reference") (OtherComp :type "PrimitiveComponent Object Reference") (NormalImpulse :type "Vector Structure") (Hit :type "HitResult Structure (by ref)"))
  (cast `/Game/Blueprints/BP_AIBall` OtherActor))

(fn `ChangeReceiver`
  (set `self.PlayerOneIsReceiver` (not (`self.PlayerOneIsReceiver`))))

(fn `FirstUp`
  (set `self.ScoreOne` (+ (`self.ScoreOne`) 1))
  (bind _asbp_game_default_game_mode (cast `/Game/Blueprints/BP_GameDefaultGameMode` (`GameplayStatics.GetGameMode`)))
  (`/Game/Blueprints/BP_GameDefaultGameMode.SetFirstScore` _asbp_game_default_game_mode (`self.ScoreOne`)))

(fn `ReseiverLose`
  (if (`self.PlayerOneIsReceiver`)
    (`self.SecondUp`)
    (else
      (`self.FirstUp`))))

(fn `SecondUp`
  (set `self.ScoreTwo` (+ (`self.ScoreTwo`) 1))
  (bind _asbp_game_default_game_mode (cast `/Game/Blueprints/BP_GameDefaultGameMode` (`GameplayStatics.GetGameMode`)))
  (`/Game/Blueprints/BP_GameDefaultGameMode.SetSecondScore` _asbp_game_default_game_mode (`self.ScoreTwo`)))

(fn `SpawnNewBall`
  (bind (_returnvalue_location _returnvalue_rotation) (`KismetMathLibrary.BreakTransform` (`self.GetTransform`)))
  (bind _returnvalue (`|SpawnActorFromClass` (`self.BallType`) (`KismetMathLibrary.MakeTransform` (+ _returnvalue_location (`KismetMathLibrary.MakeVector` -10.0 (`KismetMathLibrary.Conv_IntToDouble` (- (`KismetMathLibrary.RandomInteger` 200) 100)) 200.0)) _returnvalue_rotation) "Undefined" "OverrideRootScale" null null))
  (bind _asbp_ball (cast `/Game/Blueprints/BP_Ball` _returnvalue)
    (:`then`
      (set `/Game/Blueprints/BP_Ball.ParentTable` self _asbp_ball)
      (`/Game/Blueprints/BP_Ball.EnterTriggerOne` _asbp_ball))
    (:`CastFailed`
      (bind _asbp_aiball (cast `/Game/Blueprints/BP_AIBall` _returnvalue))
      (set `/Game/Blueprints/BP_AIBall.ParentTable` self _asbp_aiball)
      (`/Game/Blueprints/BP_AIBall.EnterTriggerOne` _asbp_aiball)))
  (set `self.PlayerOneIsReceiver` true))

(fn `ThrowerLose`
  (if (`self.PlayerOneIsReceiver`)
    (`self.FirstUp`)
    (else
      (`self.SecondUp`))))

(fn `UserConstructionScript`)