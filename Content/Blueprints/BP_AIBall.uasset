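; Table-tennis ball that scores player rocket hits and asks its parent table for a replacement when play ends.
; It launches with randomized velocity, then hit events drive a state machine alternating between flying to a rocket and to the opposite table side, tracked by triggers.
; Valid landings send the 2D distance from the rocket's target to that rocket's controller.
; Bad landings or leaving the table after a hit send a penalty.
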(event `self.ReceiveBeginPlay`
  (set `self.VelocityVector` (`KismetMathLibrary.GreaterGreater_VectorRotator` (`KismetMathLibrary.MakeVector` (`KismetMathLibrary.RandomFloatInRange` 1.0 5.0)) (`KismetMathLibrary.MakeRotator` 0.0 (`KismetMathLibrary.RandomFloatInRange` -30.0) (`KismetMathLibrary.RandomFloatInRange` -30.0 30.0)))))

(event `self.BaseMesh.OnComponentHit`
  (params (HitComponent :type "PrimitiveComponent Object Reference") (OtherActor :type "Actor Object Reference") (OtherComp :type "PrimitiveComponent Object Reference") (NormalImpulse :type "Vector Structure") (Hit :type "HitResult Structure (by ref)"))
  (`self.ChangeState` OtherActor))

(fn `CalculateResult`
  (returns (Result :type Integer))
  (bind (_returnvalue_x _returnvalue_y) (`KismetMathLibrary.BreakVector` (`self.K2_GetActorLocation`)))
  (bind _target (`PlayerRocket.Target` (`self.LastRocket`)))
  (bind (_returnvalue_x_2 _returnvalue_y_2) (`KismetMathLibrary.BreakVector` (`self.K2_GetActorLocation` _target)))
  (if (`KismetSystemLibrary.IsValid` _target)
    (return (`KismetMathLibrary.FTrunc` (`KismetMathLibrary.Distance2D` (`KismetMathLibrary.MakeVector2D` _returnvalue_x_2 _returnvalue_y_2) (`KismetMathLibrary.MakeVector2D` _returnvalue_x _returnvalue_y))))))

(fn `ChangeState`
  (params (Actor :type "Actor Object Reference"))
  (switch `/Game/Util/E_BallStates` (`self.State`)
    (:`NewEnumerator0`
      (bind _asbp_player_rocket (cast `/Game/Blueprints/BP_PlayerRocket` Actor)
        (:`then`
          (set `self.LastRocket` _asbp_player_rocket)
          (set `self.State` "NewEnumerator6")
          (if (`|EnumEquality` (`self.Side`) "NewEnumerator0")
            (set `self.ExpectingSide` "NewEnumerator1")
            (else
              (set `self.ExpectingSide` "NewEnumerator0"))))
        (:`CastFailed`
          (`self.EndGame`))))
    (:`NewEnumerator6`
      (cast `/Game/Blueprints/BP_Table` Actor
        (:`then`
          (if (`|EnumEquality` (`self.Side`) (`self.ExpectingSide`))
            (set `self.State` "NewEnumerator0")
            (bind _result (`self.CalculateResult`))
            (`self.SendResultToRocket` _result)
            (else
              (`self.SendResultToRocket` -50 :!label _label)
              (`self.EndGame`))))
        (:`CastFailed`
          (goto _label))))))

(fn `EndGame`
  (`/Game/Blueprints/BP_Table.SpawnNewBall` (`self.ParentTable`))
  (`self.K2_DestroyActor`))

(fn `EnterTriggerOne`
  (set `self.Side` "NewEnumerator0"))

(fn `EnterTriggerTwo`
  (set `self.Side` "NewEnumerator1"))

(fn `Net`)

(fn `OutOfTable`
  (if (not (`self.IsActorBeingDestroyed`))
    (if (`|EnumEquality` (`self.State`) "NewEnumerator6")
      (`self.SendResultToRocket` -50))
    (`self.EndGame`)))

(fn `SendResultToRocket`
  (params (Result :type Integer))
  (`PlayerRocket.SendControllerHittingResult` (`self.LastRocket`) Result))

(fn `UserConstructionScript`)