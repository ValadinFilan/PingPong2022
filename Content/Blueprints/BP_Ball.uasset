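; BP_Ball is the ball in a table-tennis style game that enforces the bounce rules and decides who loses the point.
; Each mesh hit advances a state machine from serve through table bounces to racket returns, checking the table side set by trigger functions against the expected side.
; An invalid hit or leaving the table makes BP_Table penalize the thrower or receiver by state, spawn a new ball and destroy this one.
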(event `self.ReceiveBeginPlay`)

(event `self.BaseMesh.OnComponentHit`
  (params (HitComponent :type "PrimitiveComponent Object Reference") (OtherActor :type "Actor Object Reference") (OtherComp :type "PrimitiveComponent Object Reference") (NormalImpulse :type "Vector Structure") (Hit :type "HitResult Structure (by ref)"))
  (`self.ChangeState` OtherActor))

(fn `ChangeState`
  (params (Actor :type "Actor Object Reference"))
  (switch `/Game/Util/E_BallStates` (`self.State`)
    (:`NewEnumerator4`
      (cast `/Game/Blueprints/BP_PlayerRocket` Actor
        (:`then`
          (set `self.State` "NewEnumerator1")
          (set `self.ExpectingSide` (`self.Side`))
          (`/Game/Blueprints/BP_Table.ChangeReceiver` (`self.ParentTable`)))
        (:`CastFailed`
          (`self.EndGame`))))
    (:`NewEnumerator0`
      (cast `/Game/Blueprints/BP_PlayerRocket` Actor
        (:`then`
          (set `self.State` "NewEnumerator6")
          (`/Game/Blueprints/BP_Table.ChangeReceiver` (`self.ParentTable`))
          (if (`|EnumEquality` (`self.Side`) "NewEnumerator0")
            (set `self.ExpectingSide` "NewEnumerator1")
            (else
              (set `self.ExpectingSide` "NewEnumerator0"))))
        (:`CastFailed`
          (`self.EndGame`))))
    (:`NewEnumerator1`
      (cast `/Game/Blueprints/BP_Table` Actor)
      (if (`|EnumEquality` (`self.Side`) (`self.ExpectingSide`))
        (set `self.State` "NewEnumerator6")
        (if (`|EnumEquality` (`self.Side`) "NewEnumerator0")
          (set `self.ExpectingSide` "NewEnumerator1")
          (else
            (set `self.ExpectingSide` "NewEnumerator0")))
        (else
          (`self.EndGame`))))
    (:`NewEnumerator6`
      (cast `/Game/Blueprints/BP_Table` Actor)
      (if (`|EnumEquality` (`self.Side`) (`self.ExpectingSide`))
        (set `self.State` "NewEnumerator0")
        (else
          (`self.EndGame`))))))

(fn `EndGame`
  (bind _parenttable (`self.ParentTable`))
  (switch `/Game/Util/E_BallStates` (`self.State`)
    (:`NewEnumerator4`
      (`/Game/Blueprints/BP_Table.ReseiverLose` _parenttable :!label _label))
    (:`NewEnumerator0`
      (goto _label))
    (:`NewEnumerator1`
      (`/Game/Blueprints/BP_Table.ThrowerLose` _parenttable :!label _label_2))
    (:`NewEnumerator6`
      (goto _label_2)))
  (`/Game/Blueprints/BP_Table.SpawnNewBall` _parenttable)
  (`self.K2_DestroyActor`))

(fn `EnterTriggerOne`
  (set `self.Side` "NewEnumerator0"))

(fn `EnterTriggerTwo`
  (set `self.Side` "NewEnumerator1"))

(fn `OutOfTable`
  (if (not (`self.IsActorBeingDestroyed`))
    (`self.EndGame`)))

(fn `UserConstructionScript`)